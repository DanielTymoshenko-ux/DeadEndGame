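; BP_Zombie is a wave-mode enemy that chases the player and attacks in melee.
; It loops AIMoveTo and an attack montage, whose notify runs a sphere overlap at Arrow1 to damage BP_Character.
; Pawn sensing sets its chase speed on sight.
; Damage reduces Health and plays a reaction, or triggers death, which disables collision, reports the kill to Zombie_Wave_Mode and destroys the actor after a delay.
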(event `self.ReceiveBeginPlay`
  (`self.run_to_player`))

(event `run_to_player`
  (if (not (`self.IsDead?`))
    (`|AIMoveTo` self (0.0 0.0 0.0) (`GameplayStatics.GetPlayerController` 0) 40.0
      (:`OnSuccess`
        (`self.AttackPlayer`))
      (:`OnFail`
        (`self.run_to_player`)))))

(event `self.PawnSensing.OnSeePawn`
  (params (Pawn :type "Pawn Object Reference"))
  (set `CharacterMovementComponent.MaxWalkSpeed` 360.0 (`self.CharacterMovement`)))

(event `AttackPlayer`
  (`|PlayMontage` (`self.Mesh`) "/Game/FPS_Tut/Zombie/Animations/Zombie_AttackM1.Zombie_AttackM1"
    (:`OnCompleted`
      (`self.run_to_player`))
    (:`OnNotifyBegin`
      (bind (_outactors _returnvalue) (`KismetSystemLibrary.SphereOverlapActors` (`SceneComponent.K2_GetComponentLocation` (`self.Arrow1`)) 80.0 (`|MakeArray` "ObjectTypeQuery3" :!type "EObjectTypeQuery Enum") "/Game/FPS_Tut/Core/BP_Character.BP_Character_C" (`|MakeArray` self :!type "Actor Object Reference")))
      (if _returnvalue
        (for _array_element _outactors
          (`GameplayStatics.ApplyDamage` _array_element 20.0 (`self.GetController`) self "/Script/Engine.DamageType"))))))

(event `self.ReceiveAnyDamage`
  (params (Damage :type "Float (single-precision)") (DamageType :type "DamageType Object Reference") (InstigatedBy :type "Controller Object Reference") (DamageCauser :type "Actor Object Reference"))
  (if (`self.IsDead?`)
    _
    (elif (<= (`self.Health`) 0.0)
      (`self.Death`)
      (`KismetSystemLibrary.Delay` 5.0 :!label _label)
      (else
        (bind _output_get (set `self.Health` (- (`self.Health`) Damage)))
        (`KismetSystemLibrary.PrintString` (`KismetStringLibrary.Conv_DoubleToString` _output_get))
        (if (<= _output_get 0.0)
          (`self.Death`)
          (goto _label)
          (else
            (`|PlayMontage` (`self.Mesh`) "/Game/FPS_Tut/Zombie/Animations/Zombie_REACT_Montage.Zombie_REACT_Montage")))))))

(event `Death`
  (set `self.IsDead?` true)
  (`MovementComponent.StopMovementImmediately` (`self.CharacterMovement`))
  (`|PlayMontage` (`self.Mesh`) "/Game/FPS_Tut/Zombie/Animations/Montage_Death_Zombie.Montage_Death_Zombie"
    (:`then`
      (`PrimitiveComponent.SetCollisionResponseToChannel` (`self.CapsuleComponent`) "ECC_Pawn" "ECR_Overlap")
      (`PrimitiveComponent.SetCollisionEnabled` (`self.CapsuleComponent`) "NoCollision")
      (bind _aszombie_wave_mode (cast `/Game/FPS_Tut/Core/Zombie_Wave_Mode` (`GameplayStatics.GetGameMode`)))
      (`/Game/FPS_Tut/Core/Zombie_Wave_Mode.Zmbie_Killed` _aszombie_wave_mode)
      (`KismetSystemLibrary.Delay` 10.0)
      (`self.K2_DestroyActor`))))

(fn `UserConstructionScript`)