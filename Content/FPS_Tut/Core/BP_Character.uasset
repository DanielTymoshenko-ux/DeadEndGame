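; BP_Character is the first-person shooter player character, handling Enhanced Input movement, sprint with FOV timeline, jump, aim flag, shooting and grenades.
; BeginPlay creates the HUD and spawns inventory weapons on the arms' hand socket, showing the equipped one.
; Rifle fire loops on a delay, spawning BP_Bullet, and is blocked while running, reloading or near walls detected by a Tick trace.
; It also tracks both ammo pools, crate pickups, damage, death and timer-based regeneration.
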(event `EnhancedInput|/Game/FPS_Tut/Data/IA_Reload`
  (params (ActionValue :type Boolean) (ElapsedSeconds :type "Float (double-precision)") (TriggeredSeconds :type "Float (double-precision)") (InputAction :type "InputAction Object Reference" :default "/Game/FPS_Tut/Data/IA_Reload.IA_Reload")))

(event `EnhancedInput|/Game/FPS_Tut/Data/IA_Reload1_Grenade`
  (params (ActionValue :type Boolean) (ElapsedSeconds :type "Float (double-precision)") (TriggeredSeconds :type "Float (double-precision)") (InputAction :type "InputAction Object Reference" :default "/Game/FPS_Tut/Data/IA_Reload1_Grenade.IA_Reload1_Grenade"))
  (bind _returnvalue (+ (`self.TotalAmmunition_Grenade`) (`self.CurrentAmmunition_Grenade`)))
  (bind _returnvalue_2 (>= _returnvalue (`self.ClipSize_Grenade`)))
  (:`Triggered`
    ;[1 1 1] Reload
    (`/Engine/EditorBlueprintResources/StandardMacros.DoOnce` false :!label _label
      (:`Completed`
        (if (or (== (`self.CurrentAmmunition_Grenade`) (`self.ClipSize_Grenade`)) (<= (`self.TotalAmmunition_Grenade`) 0))
          (set `self.b_reloading` false)
          (else
            (set `self.b_reloading` true)
            (set `self.TempAmmo_Grenade` (`self.CurrentAmmunition_Grenade`))
            (set `self.CurrentAmmunition_Grenade` (`KismetMathLibrary.SelectInt` (`self.ClipSize_Grenade`) _returnvalue _returnvalue_2))
            (set `self.TotalAmmunition_Grenade` (`KismetMathLibrary.SelectInt` (`KismetMathLibrary.Clamp` (- (`self.TotalAmmunition_Grenade`) (- (`self.ClipSize_Grenade`) (`self.TempAmmo_Grenade`))) 0 (`self.TotalAmmunition_Grenade`)) 0 _returnvalue_2))
            (message `/Game/FPS_Tut/Core/BPI_Weapon.Reload` (`|GetArrayItem` (`self.EquipedWeapons`) (`self.EquipedWeaponIndex`)))
            (`GameplayStatics.SpawnSound2D` "/Game/FPS_Tut/Core/m4a1-or-m16-reload-sound-84436.m4a1-or-m16-reload-sound-84436" 1.0 1.0 0.0 null)
            (`KismetSystemLibrary.Delay` 2.0))))))
  (:`Completed`
    (goto _label :!via `Reset`)))

(event `GetAmmoCrate_Grenade`
  ;[1 1 1] PickUpAmmo
  (set `self.CurrentAmmunition_Grenade` (+ (`self.CurrentAmmunition_Grenade`) 1))
  (`GameplayStatics.PlaySound2D` "/Game/FPS_Tut/Core/crate-break-1-93926.crate-break-1-93926" 1.0 1.0 0.0 null null))

(event `EnhancedInput|/Game/FPS_Tut/Data/IA_Reload`
  (params (ActionValue :type Boolean) (ElapsedSeconds :type "Float (double-precision)") (TriggeredSeconds :type "Float (double-precision)") (InputAction :type "InputAction Object Reference" :default "/Game/FPS_Tut/Data/IA_Reload.IA_Reload"))
  (bind _returnvalue (+ (`self.TotalAmmunition`) (`self.CurrentAmmunition`)))
  (bind _returnvalue_2 (>= _returnvalue (`self.ClipSize`)))
  ;[1 1 1] Reload
  (:`Triggered`
    (`/Engine/EditorBlueprintResources/StandardMacros.DoOnce` false :!label _label_2
      (:`Completed`
        (if (or (== (`self.CurrentAmmunition`) (`self.ClipSize`)) (<= (`self.TotalAmmunition`) 0))
          (set `self.b_reloading` false)
          (else
            (set `self.b_reloading` true)
            (set `self.TempAmmo` (`self.CurrentAmmunition`))
            (set `self.CurrentAmmunition` (`KismetMathLibrary.SelectInt` (`self.ClipSize`) _returnvalue _returnvalue_2))
            (set `self.TotalAmmunition` (`KismetMathLibrary.SelectInt` (`KismetMathLibrary.Clamp` (- (`self.TotalAmmunition`) (- (`self.ClipSize`) (`self.TempAmmo`))) 0 (`self.TotalAmmunition`)) 0 _returnvalue_2))
            (`|PlayMontage` (`self.CharacterArms`) "/Game/FPS_Tut/Art/Assault_Rifle/Animaitons/AM_FP_AssaultRifle_Reload_.AM_FP_AssaultRifle_Reload_"
              (:`then`
                (message `/Game/FPS_Tut/Core/BPI_Weapon.Reload` (`|GetArrayItem` (`self.EquipedWeapons`) (`self.EquipedWeaponIndex`)))
                (`GameplayStatics.SpawnSound2D` "/Game/FPS_Tut/Core/m4a1-or-m16-reload-sound-84436.m4a1-or-m16-reload-sound-84436" 1.0 1.0 0.0 null)
                (`KismetSystemLibrary.Delay` 2.0))
              (:`OnBlendOut`
                (set `self.b_reloading` false))))))))
  (:`Completed`
    (goto _label_2 :!via `Reset`)))

(event `GetAmmoCrate`
  ;[1 1 1] PickUpAmmo
  (set `self.CurrentAmmunition` (`self.ClipSize`))
  (set `self.TotalAmmunition` (+ (`self.TotalAmmunition`) 60))
  (`GameplayStatics.PlaySound2D` "/Game/FPS_Tut/Core/crate-break-1-93926.crate-break-1-93926" 1.0 1.0 0.0 null null))

(event `EnhancedInput|/Game/FPS_Tut/Data/IA_Shoot`
  (params (ActionValue :type Boolean) (ElapsedSeconds :type "Float (double-precision)") (TriggeredSeconds :type "Float (double-precision)") (InputAction :type "InputAction Object Reference" :default "/Game/FPS_Tut/Data/IA_Shoot.IA_Shoot"))
  (bind _returnvalue (and (and (and (`self.B_HoldingShoot`) (not (`self.b_closeToWall`)) (not (`self.b_running`))) (> (`self.CurrentAmmunition`) 0)) (`KismetMathLibrary.BooleanNOR` (`self.b_reloading`))))
  (:`Triggered`
    (`/Engine/EditorBlueprintResources/StandardMacros.DoOnce` false :!label _label_3
      (:`Completed`
        (set `self.B_HoldingShoot` true)
        (if _returnvalue
          (if _returnvalue :!label _label_4
            (`|PlayMontage` (`self.CharacterArms`) "/Game/FPS_Tut/Art/Assault_Rifle/Animaitons/AM_FP_Assault_Rifle_Fire.AM_FP_Assault_Rifle_Fire"
              (:`then`
                (bind _returnvalue_2 (`|SpawnActorFromClass` "/Game/FPS_Tut/Core/BP_Bullet.BP_Bullet_C" (`SceneComponent.K2_GetComponentToWorld` (`self.Arrow1`)) "AlwaysSpawn" "MultiplyWithRoot" null null))
                (`PrimitiveComponent.IgnoreActorWhenMoving` (`self.CapsuleComponent`) null true)
                (`PrimitiveComponent.IgnoreActorWhenMoving` (`/Game/FPS_Tut/Core/BP_Bullet.Sphere` _returnvalue_2) self true)
                (`GameplayStatics.SpawnEmitterAttached` "/Game/MilitaryWeapSilver/FX/P_AssaultRifle_MuzzleFlash.P_AssaultRifle_MuzzleFlash" (`Actor.RootComponent` (`|GetArrayItem` (`self.EquipedWeapons`) (`self.EquipedWeaponIndex`))) "None" (0.0 100.0 0.0) (struct) (0.02 0.02 0.02) "SnapToTargetIncludingScale")
                (set `self.CurrentAmmunition` (- (`self.CurrentAmmunition`) 1))
                (`GameplayStatics.PlaySound2D` "/Game/FPS_Tut/Core/assaultrifle2-47258.assaultrifle2-47258" 1.0 1.0 0.0 null null)
                (`KismetSystemLibrary.LineTraceSingle` :`End` (* (`KismetMathLibrary.GetForwardVector` (struct)) (`self.bullet distance`)) :`TraceChannel` "TraceTypeQuery2" :`DrawDebugType` "Persistent")
                (`KismetSystemLibrary.Delay` (`self.FireDelay`))
                (goto _label_4))))
          (else
            (`GameplayStatics.PlaySound2D` "/Game/FPS_Tut/Core/clip-in-106657.clip-in-106657" 1.0 1.0 0.0 null null))))))
  (:`Completed`
    (set `self.B_HoldingShoot` false)
    (goto _label_3 :!via `Reset`)))

(event `EnhancedInput|/Game/FPS_Tut/Data/IA_grenade`
  (params (ActionValue :type Boolean) (ElapsedSeconds :type "Float (double-precision)") (TriggeredSeconds :type "Float (double-precision)") (InputAction :type "InputAction Object Reference" :default "/Game/FPS_Tut/Data/IA_grenade.IA_grenade"))
  ;[1 1 1] Grenade
  (:`Triggered`
    (`/Engine/EditorBlueprintResources/StandardMacros.DoOnce` false :!label _label_5
      (:`Completed`
        (set `self.B_HoldingShoot` true)
        (if (and (and (and (`self.B_HoldingShoot`) (not (`self.b_closeToWall`)) (not (`self.b_running`))) (> (`self.CurrentAmmunition_Grenade`) 0)) (`KismetMathLibrary.BooleanNOR` (`self.b_reloading`)))
          (if true
            (`|SpawnActorFromClass` "/Game/FPS_Tut/Core/Grenade/Grenade1.Grenade1_C" (`SceneComponent.K2_GetComponentToWorld` (`self.Arrow1`)) "Undefined" "MultiplyWithRoot" null null)
            (bind _output_get (set `self.CurrentAmmunition_Grenade` (- (`self.CurrentAmmunition_Grenade`) 1)))
            (`KismetSystemLibrary.PrintString` (`KismetStringLibrary.Conv_IntToString` _output_get) true true (struct :`R` 1.0 :`B` 0.029038 :`A` 1.0)))
          (else
            (`GameplayStatics.PlaySound2D` "/Game/FPS_Tut/Core/clip-in-106657.clip-in-106657" 1.0 1.0 0.0 null null))))))
  (:`Completed`
    (set `self.B_HoldingShoot` false)
    (goto _label_5 :!via `Reset`)))

(event `self.ReceiveBeginPlay`
  ;[1 1 1] Create UI
  (`EnhancedInputSubsystemInterface.AddMappingContext` (pcsubsystem `EnhancedInputLocalPlayerSubsystem` (`GameplayStatics.GetPlayerController` 0)) "/Game/FPS_Tut/Data/IMC_FPS.IMC_FPS" 0 (struct))
  (`self.SpawnInventory`)
  (bind _returnvalue (`|CreateWidget` "/Game/FPS_Tut/Core/WBP_UI.WBP_UI_C" (`GameplayStatics.GetPlayerController` 0)))
  (`UserWidget.AddToViewport` _returnvalue 0))

(event `EnhancedInput|/Game/FPS_Tut/Data/IA_Camera`
  (params (ActionValue :type "Vector2D Structure") (ElapsedSeconds :type "Float (double-precision)") (TriggeredSeconds :type "Float (double-precision)") (InputAction :type "InputAction Object Reference" :default "/Game/FPS_Tut/Data/IA_Camera.IA_Camera"))
  (bind (_x _y) (`KismetMathLibrary.BreakVector2D` (`self.MouseInput`)))
  ;[1 1 1] Cmera
  (:`Triggered`
    (set `self.MouseInput` ActionValue :!label _label_6)
    (`self.AddControllerPitchInput` (* _y -1.0))
    (`self.AddControllerYawInput` _x))
  (:`Completed`
    (goto _label_6)))

(event `EnhancedInput|/Game/FPS_Tut/Data/IA_test`
  (params (ActionValue :type Boolean) (ElapsedSeconds :type "Float (double-precision)") (TriggeredSeconds :type "Float (double-precision)") (InputAction :type "InputAction Object Reference" :default "/Game/FPS_Tut/Data/IA_test.IA_test"))
  (:`Triggered`
    (`KismetSystemLibrary.PrintString` "Hello")))

(event `EnhancedInput|/Game/FPS_Tut/Data/IA_Movement`
  (params (ActionValue :type "Vector2D Structure") (ElapsedSeconds :type "Float (double-precision)") (TriggeredSeconds :type "Float (double-precision)") (InputAction :type "InputAction Object Reference" :default "/Game/FPS_Tut/Data/IA_Movement.IA_Movement"))
  (bind (_x _y) (`KismetMathLibrary.BreakVector2D` (`self.moveInput`)))
  (:`Triggered`
    (set `self.moveInput` ActionValue :!label _label_7)
    (`self.AddMovementInput` (* (`self.GetActorRightVector`) _x))
    (`self.AddMovementInput` (* (`self.GetActorForwardVector`) _y)))
  (:`Canceled`
    (goto _label_7)))

(event `self.ReceiveRadialDamage`
  (params (DamageReceived :type "Float (single-precision)") (DamageType :type "DamageType Object Reference") (Origin :type "Vector Structure") (HitInfo :type "HitResult Structure (by ref)") (InstigatedBy :type "Controller Object Reference") (DamageCauser :type "Actor Object Reference"))
  (if (not (`self.isDead?`))
    (bind _output_get (set `self.Health` (- (`self.Health`) DamageReceived)))
    (if (<= _output_get 0.0)
      (`KismetSystemLibrary.PrintString` (`KismetStringLibrary.Conv_DoubleToString` _output_get))
      (`self.PlayerDeath`)
      (elif (<= (`self.Health`) 90.0)
        (`self.HealthRegenTimer`)
        (elif (<= (`self.Health`) 60.0)
          _)))))

(event `self.ReceiveAnyDamage`
  (params (Damage :type "Float (single-precision)") (DamageType :type "DamageType Object Reference") (InstigatedBy :type "Controller Object Reference") (DamageCauser :type "Actor Object Reference"))
  (if (not (`self.isDead?`))
    (bind _output_get (set `self.Health` (- (`self.Health`) Damage)))
    (if (<= _output_get 0.0)
      (`KismetSystemLibrary.PrintString` (`KismetStringLibrary.Conv_DoubleToString` _output_get))
      (`self.PlayerDeath`)
      (elif (<= (`self.Health`) 90.0)
        (`self.HealthRegenTimer`)
        (elif (<= (`self.Health`) 60.0)
          _)))))

(event `EnhancedInput|/Game/FPS_Tut/Data/IA_Run`
  (params (ActionValue :type Boolean) (ElapsedSeconds :type "Float (double-precision)") (TriggeredSeconds :type "Float (double-precision)") (InputAction :type "InputAction Object Reference" :default "/Game/FPS_Tut/Data/IA_Run.IA_Run"))
  (:`Triggered`
    (if (not (`NavMovementComponent.IsFalling` (`self.CharacterMovement`)))
      (set `self.b_running` true)
      (set `CharacterMovementComponent.MaxWalkSpeed` (`self.Running_Speed`) (`self.CharacterMovement`))
      (bind (_direction _fov) (`Timeline|Timeline` :!label _label_8)
        (:`Update`
          (set `PlayerCameraManager.DefaultFOV` _fov (`GameplayStatics.GetPlayerCameraManager` 0))))))
  (:`Completed`
    (`self.Stop_Running`)))

(event `Stop_Running`
  (set `self.b_running` false)
  (set `CharacterMovementComponent.MaxWalkSpeed` 300.0 (`self.CharacterMovement`))
  (goto _label_8 :!via `Reverse`))

(event `self.ReceiveTick`
  (params (DeltaSeconds :type "Float (single-precision)"))
  (bind _camera (`self.Camera`))
  (bind _returnvalue (`SceneComponent.K2_GetComponentLocation` _camera))
  (`SceneComponent.K2_SetRelativeRotation` (`self.Pivot`) (`KismetMathLibrary.MakeRotator` 0.0 (.pitch (`self.GetControlRotation`))) false false)
  (bind (_outhit _returnvalue_2) (`KismetSystemLibrary.LineTraceSingle` _returnvalue (+ _returnvalue (* (`SceneComponent.GetForwardVector` _camera) (100.0 100.0 100.0))) "TraceTypeQuery1"))
  (set `self.b_closeToWall` _returnvalue_2))

(event `EnhancedInput|/Game/FPS_Tut/Data/IA_Jumping`
  (params (ActionValue :type Boolean) (ElapsedSeconds :type "Float (double-precision)") (TriggeredSeconds :type "Float (double-precision)") (InputAction :type "InputAction Object Reference" :default "/Game/FPS_Tut/Data/IA_Jumping.IA_Jumping"))
  (:`Triggered`
    (`self.Jump`)
    (`self.Stop_Running`))
  (:`Completed`
    (`self.StopJumping`)))

(event `PlayerDeath`
  ;[1 1 1] Player_Death
  (set `self.isDead?` true))

(event `HealthRegenTimer`
  ;[1 1 1] Regeneration
  (`KismetSystemLibrary.K2_SetTimerDelegate` (delegate `Regeneration_Event`) 5.0 true))

(event `EnhancedInput|/Game/FPS_Tut/Data/IA_Aiming`
  (params (ActionValue :type Boolean) (ElapsedSeconds :type "Float (double-precision)") (TriggeredSeconds :type "Float (double-precision)") (InputAction :type "InputAction Object Reference" :default "/Game/FPS_Tut/Data/IA_Aiming.IA_Aiming"))
  ;[1 1 1] Aiming
  (:`Triggered`
    (set `self.B_Aiming` true))
  (:`Completed`
    (set `self.B_Aiming` false)))

(event `Regeneration_Event`
  ;[1 1 1] Regeneration
  (if (not (== (`self.Health`) 100.0))
    (bind _output_get (set `self.Health` (`KismetMathLibrary.FClamp` (+ (`self.Health`) 5.0) 0.0 100.0)))
    (if (>= 50.0 _output_get)
      _)))

(fn `NewFunction`)

(fn `SpawnInventory`
  (for _array_element (`self.Inventory`)
    (bind _returnvalue (`|SpawnActorFromClass` _array_element (`KismetMathLibrary.MakeTransform` (0.0 0.0 0.0)) "Undefined" "MultiplyWithRoot" null null))
    (`KismetArrayLibrary.Array_Add` (`self.EquipedWeapons`) _returnvalue)
    (`self.K2_AttachToComponent` _returnvalue (`self.CharacterArms`) "ik_hand_gun" "SnapToTarget" "SnapToTarget" "KeepRelative" true)
    (`self.SetActorHiddenInGame` _returnvalue true))
  (`self.SetActorHiddenInGame` (`|GetArrayItem` (`self.EquipedWeapons`) (`self.EquipedWeaponIndex`)) false))

(fn `UserConstructionScript`)