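; BP_Bullet is an FPS projectile that deals flat damage and destroys itself on its first Sphere component hit.
; The hit spawns a tiny explosion and an FS_MasterFIeld_Bullet field actor, triggered through CETrigger, before applying damage.
; A "Zombie" actor tag selects blood or asphalt particles, though another blood emitter always spawns afterward.
; Surface-based headshot damage and physics impulse logic are present but unconnected.
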(event `OnActorHit_Event` :!signature `self.OnActorHit`
  (params (SelfActor :type "Actor Object Reference") (OtherActor :type "Actor Object Reference") (NormalImpulse :type "Vector Structure") (Hit :type "HitResult Structure (by ref)")))

(event `self.Sphere.OnComponentHit`
  (params (HitComponent :type "PrimitiveComponent Object Reference") (OtherActor :type "Actor Object Reference") (OtherComp :type "PrimitiveComponent Object Reference") (NormalImpulse :type "Vector Structure") (Hit :type "HitResult Structure (by ref)"))
  (bind (_bblockinghit _binitialoverlap _time _distance _location _impactpoint _normal _impactnormal _physmat _hitactor) (`GameplayStatics.BreakHitResult` Hit))
  (bind _returnvalue (`self.K2_GetActorLocation`))
  (set `self.HitActor` OtherActor)
  (`/Engine/EditorBlueprintResources/StandardMacros.DoOnce` false
    (:`Completed`
      (`GameplayStatics.SpawnEmitterAtLocation` "/Game/StarterContent/Particles/P_Explosion.P_Explosion" (`self.K2_GetActorLocation`) (struct) (0.001 0.001 0.001))
      (bind _returnvalue_2 (`|SpawnActorFromClass` "/Game/FPS_Tut/Core/FS_MasterFIeld_Bullet.FS_MasterFIeld_Bullet_C" (`self.GetTransform`) "AlwaysSpawn" "MultiplyWithRoot" null null))
      (set `self.Field` _returnvalue_2)
      (`/Engine/EditorResources/FieldNodes/FS_MasterField.CE_Trigger` (`self.Field`))
      (`GameplayStatics.ApplyDamage` (`self.HitActor`) 25.0)
      (if (`self.ActorHasTag` _hitactor "Zombie")
        (`GameplayStatics.SpawnEmitterAtLocation` "/Game/Realistic_Starter_VFX_Pack_Vol2/Particles/Blood/P_Blood_Splat_Cone.P_Blood_Splat_Cone" _returnvalue)
        (else
          (`GameplayStatics.SpawnEmitterAtLocation` "/Game/Realistic_Starter_VFX_Pack_Vol2/Particles/Hit/P_Asphalt.P_Asphalt" _location)))
      (`GameplayStatics.SpawnEmitterAttached` "/Game/Realistic_Starter_VFX_Pack_Vol2/Particles/Blood/P_Blood_Splat_Cone.P_Blood_Splat_Cone" null "None" _returnvalue)
      (`self.K2_DestroyActor` self))))

(fn `UserConstructionScript`)